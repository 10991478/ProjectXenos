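; Test Blueprint for automatic double doors that slide along local X when something overlaps their Collider.
; The overlap sets a never-cleared DoorsInMotion latch before the Character cast, then plays a close or open timeline based on DoorsAreOpen, which is never changed here.
; MoveDoors offsets both doors oppositely from Door01's stored location with sweep, and that location is re-captured every update, so offsets accumulate.
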(event `self.ReceiveBeginPlay`
  ;[1 1 1] Set Initial Door Locations
  (`self.SetCurrentDoorLocations`))

(event `self.Collider.OnComponentBeginOverlap`
  (params (OverlappedComponent :type "PrimitiveComponent Object Reference") (OtherActor :type "Actor Object Reference") (OtherComp :type "PrimitiveComponent Object Reference") (OtherBodyIndex :type Integer) (bFromSweep :type Boolean) (SweepResult :type "HitResult Structure (by ref)"))
  ;[1 1 1] Move the Doors when Player Hits Collider
  (if (not (`self.DoorsInMotion`))
    (set `self.DoorsInMotion` true)
    (cast `Character` OtherActor)
    (`self.SetCurrentDoorLocations`)
    (if (`self.DoorsAreOpen`)
      (bind (_direction _doorsclose) (`Timeline|Timeline` :!via `PlayFromStart`)
        (:`Update`
          (`self.MoveDoors` _doorsclose)
          (`self.SetCurrentDoorLocations`)))
      (else
        (bind (_direction_2 _doorsopen) (`Timeline|Timeline_0` :!via `PlayFromStart`)
          (:`Update`
            (`self.MoveDoors` _doorsopen)
            (`self.SetCurrentDoorLocations`)))))))

(fn `MoveDoors`
  (params (Movement :type "Float (double-precision)"))
  (bind (_door_01_start_location_x _door_01_start_location_y _door_01_start_location_z) (`KismetMathLibrary.BreakVector` (`self.Door_01_Start_Location`)))
  (bind (_door_01_start_location_x_2 _door_01_start_location_y_2 _door_01_start_location_z_2) (`KismetMathLibrary.BreakVector` (`self.Door_01_Start_Location`)))
  (`SceneComponent.K2_SetRelativeLocation` (`self.Door_01`) (`KismetMathLibrary.MakeVector` (+ _door_01_start_location_x (* (`self.DoorTravelDistance`) Movement)) _door_01_start_location_y _door_01_start_location_z) true false)
  (`SceneComponent.K2_SetRelativeLocation` (`self.Door_02`) (`KismetMathLibrary.MakeVector` (- _door_01_start_location_x_2 (* (`self.DoorTravelDistance`) Movement)) _door_01_start_location_y_2 _door_01_start_location_z_2) true false))

(fn `SetCurrentDoorLocations`
  (set `self.Door_01_Start_Location` (`SceneComponent.RelativeLocation` (`self.Door_01`)))
  (set `self.Door_02_Start_Location` (`SceneComponent.RelativeLocation` (`self.Door_02`))))

(fn `UserConstructionScript`)
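; Base double sliding door Blueprint, named as access-restricted, that slides two door meshes apart along their relative X axis.
; BeginPlay caches both meshes' start positions, and a timeline curve scaled by OpenDist offsets them in opposite directions.
; OpenDoor plays a sound and the timeline, while CloseDoor reverses it silently.
; No access check appears in these graphs.
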(event `self.ReceiveBeginPlay`
  (set `self.Door_01_StartPos` (`SceneComponent.RelativeLocation` (`self.DoorMesh_01`)))
  (set `self.Door_02_StartPos` (`SceneComponent.RelativeLocation` (`self.DoorMesh_02`))))

(event `self.OpenDoor`
  (bind (_door_01_startpos_x _door_01_startpos_y _door_01_startpos_z) (`KismetMathLibrary.BreakVector` (`self.Door_01_StartPos`)))
  (bind (_door_02_startpos_x _door_02_startpos_y _door_02_startpos_z) (`KismetMathLibrary.BreakVector` (`self.Door_02_StartPos`)))
  (`GameplayStatics.PlaySoundAtLocation` "/Game/Audio/Alien_Isolation_Sound_Files/Additional/Sound_Effects/door_double_open.door_double_open" (`self.K2_GetActorLocation`) (struct) 1.0 1.0 0.0 null null null null)
  (bind (_direction _dooranim_01) (`Timeline|Timeline` :!label _label)
    (:`Update`
      (bind _returnvalue (* _dooranim_01 (`self.OpenDist`)))
      (`SceneComponent.K2_SetRelativeLocation` (`self.DoorMesh_01`) (`KismetMathLibrary.MakeVector` (+ _returnvalue _door_01_startpos_x) _door_01_startpos_y _door_01_startpos_z) false false)
      (`SceneComponent.K2_SetRelativeLocation` (`self.DoorMesh_02`) (`KismetMathLibrary.MakeVector` (+ (* _returnvalue -1.0) _door_02_startpos_x) _door_02_startpos_y _door_02_startpos_z) false false))))

(event `self.CloseDoor`
  (goto _label :!via `Reverse`))

(fn `UserConstructionScript`
  (`parent.UserConstructionScript`))
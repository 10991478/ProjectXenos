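; Base automatic door that needs an activation signal before it opens for nearby actors.
; While unlocked, actors matching DoorOpeningClasses open it on entering the collider; their exit closes it regardless of lock state.
; ActivateSignal unlocks it, opens it if the first-person character is already inside, and sets default nav area; DeactivateSignal locks, closes and sets null nav area.
; Both signals call post-change functions.
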(event `self.DoorCollider_01.OnComponentBeginOverlap`
  (params (OverlappedComponent :type "PrimitiveComponent Object Reference") (OtherActor :type "Actor Object Reference") (OtherComp :type "PrimitiveComponent Object Reference") (OtherBodyIndex :type Integer) (bFromSweep :type Boolean) (SweepResult :type "HitResult Structure (by ref)"))
  (if (`self.IsUnlocked`)
    (`/Game/Blueprints/Macros/BML_CastToClass_Actor.CastActorToClasses` OtherActor (`self.DoorOpeningClasses`)
      (:`Passed`
        (`self.OpenDoor`)))))

(event `self.DoorCollider_01.OnComponentEndOverlap`
  (params (OverlappedComponent :type "PrimitiveComponent Object Reference") (OtherActor :type "Actor Object Reference") (OtherComp :type "PrimitiveComponent Object Reference") (OtherBodyIndex :type Integer))
  (`/Game/Blueprints/Macros/BML_CastToClass_Actor.CastActorToClasses` OtherActor (`self.DoorOpeningClasses`)
    (:`Passed`
      (`self.CloseDoor`))))

(event `/Game/Blueprints/BP_Interfaces/BPI_BasicActivationSignal.ActivateSignal`
  (`NavModifierComponent.SetAreaClass` (`self.NavModifier`) "/Script/NavigationSystem.NavArea_Default")
  (set `self.IsUnlocked` true)
  (`self.PostActivation`)
  (if (> (`KismetArrayLibrary.Array_Length` (`PrimitiveComponent.GetOverlappingActors` (`self.DoorCollider_01`) "/Game/FirstPerson/Blueprints/BP_FirstPersonCharacter.BP_FirstPersonCharacter_C")) 0)
    (`self.OpenDoor`)))

(event `/Game/Blueprints/BP_Interfaces/BPI_BasicActivationSignal.DeactivateSignal`
  (`NavModifierComponent.SetAreaClass` (`self.NavModifier`) "/Script/NavigationSystem.NavArea_Null")
  (set `self.IsUnlocked` false)
  (`self.PostDeactivation`)
  (`self.CloseDoor`))

(fn `UserConstructionScript`
  (`parent.UserConstructionScript`))
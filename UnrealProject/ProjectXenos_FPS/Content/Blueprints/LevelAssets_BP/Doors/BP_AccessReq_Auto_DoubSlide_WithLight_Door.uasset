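; Access-required automatic double sliding door Blueprint with two indicator lights that show whether the door is activated.
; The PostActivation event turns both point lights green, and PostDeactivation turns them red.
; The graph holds no door movement or access-check logic, and the construction script only calls its parent.
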(event `/Game/Blueprints/LevelAssets_BP/Doors/BP_Base_AccessReq_Auto_Door.PostActivation`
  (`LightComponent.SetLightColor` (`self.PointLight_01`) (struct :`G` 1.0 :`A` 1.0) true)
  (`LightComponent.SetLightColor` (`self.PointLight_02`) (struct :`G` 1.0 :`A` 1.0) true))

(event `/Game/Blueprints/LevelAssets_BP/Doors/BP_Base_AccessReq_Auto_Door.PostDeactivation`
  (`LightComponent.SetLightColor` (`self.PointLight_01`) (struct :`R` 1.0 :`A` 1.0) true)
  (`LightComponent.SetLightColor` (`self.PointLight_02`) (struct :`R` 1.0 :`A` 1.0) true))

(fn `UserConstructionScript`
  (`parent.UserConstructionScript`))
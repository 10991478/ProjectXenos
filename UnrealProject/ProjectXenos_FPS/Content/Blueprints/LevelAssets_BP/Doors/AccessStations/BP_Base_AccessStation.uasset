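; Base access station that opens linked doors when the interacting first-person character has sufficient clearance.
; On interact, it gets the player's access level through a message and sends an activate signal to each mapped door whose required level is met.
; OpenDoorsUsingAccessLevel repeats that check for a supplied level, and IsInteractable returns false here.
; A collider shows and hides the station's widget as the player enters and leaves.
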(event `/Game/Blueprints/BP_Interfaces/BPI_Interactable.OnInteract`
  (params (InteractingPlayer :type "Character Object Reference"))
  (bind _linkeddoorsandtheiraccesslevels (`self.LinkedDoorsAndTheirAccessLevels`))
  ;[1 1 1] Handling Button Press
  (bind _asbp_first_person_character (cast `/Game/FirstPerson/Blueprints/BP_FirstPersonCharacter` InteractingPlayer))
  (bind _accesslevel (message `/Game/Blueprints/BP_Interfaces/BPI_AccessLevel.GetAccessLevel` _asbp_first_person_character))
  (bind _keys (`BlueprintMapLibrary.Map_Keys` _linkeddoorsandtheiraccesslevels))
  (for _array_element _keys
    (if (>= _accesslevel (`BlueprintMapLibrary.Map_Find` _linkeddoorsandtheiraccesslevels _array_element))
      (message `/Game/Blueprints/BP_Interfaces/BPI_BasicActivationSignal.ActivateSignal` _array_element))))

(event `self.InteractionCollider.OnComponentBeginOverlap`
  (params (OverlappedComponent :type "PrimitiveComponent Object Reference") (OtherActor :type "Actor Object Reference") (OtherComp :type "PrimitiveComponent Object Reference") (OtherBodyIndex :type Integer) (bFromSweep :type Boolean) (SweepResult :type "HitResult Structure (by ref)"))
  ;[1 1 1] Widget Visibility
  (cast `/Game/FirstPerson/Blueprints/BP_FirstPersonCharacter` OtherActor)
  (`SceneComponent.SetVisibility` (`self.Widget_01`) true false))

(event `self.InteractionCollider.OnComponentEndOverlap`
  (params (OverlappedComponent :type "PrimitiveComponent Object Reference") (OtherActor :type "Actor Object Reference") (OtherComp :type "PrimitiveComponent Object Reference") (OtherBodyIndex :type Integer))
  ;[1 1 1] Widget Visibility
  (cast `/Game/FirstPerson/Blueprints/BP_FirstPersonCharacter` OtherActor)
  (`SceneComponent.SetVisibility` (`self.Widget_01`) false false))

(fn `IsInteractable`
  (returns (Interactable :type Boolean))
  (return false))

(fn `OpenDoorsUsingAccessLevel`
  (params (`Access Level` :type Integer))
  (bind _linkeddoorsandtheiraccesslevels (`self.LinkedDoorsAndTheirAccessLevels`))
  (bind _keys (`BlueprintMapLibrary.Map_Keys` _linkeddoorsandtheiraccesslevels))
  (for _array_element _keys
    (if (>= `Access Level` (`BlueprintMapLibrary.Map_Find` _linkeddoorsandtheiraccesslevels _array_element))
      (message `/Game/Blueprints/BP_Interfaces/BPI_BasicActivationSignal.ActivateSignal` _array_element))))

(fn `UserConstructionScript`)
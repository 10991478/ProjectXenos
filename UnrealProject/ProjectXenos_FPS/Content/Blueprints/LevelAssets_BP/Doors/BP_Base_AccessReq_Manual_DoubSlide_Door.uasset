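; Base Blueprint for a manual, access-requirement double sliding door that moves two door meshes apart to open.
; On BeginPlay it stores both meshes' starting relative locations.
; OpenDoor plays a timeline whose curve, scaled by OpenDist, offsets the meshes in opposite directions along local X, and CloseDoor reverses it.
; No access check appears in this graph, only the slide motion.
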(event `self.ReceiveBeginPlay`
  (`parent.ReceiveBeginPlay`)
  (set `self.Door_01_StartPos` (`SceneComponent.RelativeLocation` (`self.DoorMesh_01`)))
  (set `self.Door_02_StartPos` (`SceneComponent.RelativeLocation` (`self.DoorMesh_02`))))

(event `self.OpenDoor`
  (bind (_door_01_startpos_x _door_01_startpos_y _door_01_startpos_z) (`KismetMathLibrary.BreakVector` (`self.Door_01_StartPos`)))
  (bind (_door_02_startpos_x _door_02_startpos_y _door_02_startpos_z) (`KismetMathLibrary.BreakVector` (`self.Door_02_StartPos`)))
  (bind (_direction _dooranim_01) (`Timeline|Timeline` :!label _label)
    (:`Update`
      (bind _returnvalue (* _dooranim_01 (`self.OpenDist`)))
      (`SceneComponent.K2_SetRelativeLocation` (`self.DoorMesh_01`) (`KismetMathLibrary.MakeVector` (+ _returnvalue _door_01_startpos_x) _door_01_startpos_y _door_01_startpos_z) false false)
      (`SceneComponent.K2_SetRelativeLocation` (`self.DoorMesh_02`) (`KismetMathLibrary.MakeVector` (+ (* _returnvalue -1.0) _door_02_startpos_x) _door_02_startpos_y _door_02_startpos_z) false false))))

(event `self.CloseDoor`
  (goto _label :!via `Reverse`))

(fn `UserConstructionScript`
  (`parent.UserConstructionScript`))
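; Double sliding door Blueprint that moves two door meshes apart along their local X axis on OpenDoor and back on CloseDoor.
; BeginPlay caches both relative locations, and a timeline scales OpenDist to offset the meshes in opposite directions, reversing to close.
; The cached positions are crossed, so each mesh animates from the other's start location.
; No trigger logic appears in these graphs.
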(event `self.ReceiveBeginPlay`
  (set `self.Door02StartPos` (`SceneComponent.RelativeLocation` (`self.DoorMesh_01`)))
  (set `self.Door01StartPos` (`SceneComponent.RelativeLocation` (`self.DoorMesh_02`))))

(event `self.OpenDoor`
  (bind (_door01startpos_x _door01startpos_y _door01startpos_z) (`KismetMathLibrary.BreakVector` (`self.Door01StartPos`)))
  (bind (_door02startpos_x _door02startpos_y _door02startpos_z) (`KismetMathLibrary.BreakVector` (`self.Door02StartPos`)))
  (bind (_direction _dooranim_01) (`Timeline|Timeline` :!label _label)
    (:`Update`
      (bind _returnvalue (* _dooranim_01 (`self.OpenDist`)))
      (`SceneComponent.K2_SetRelativeLocation` (`self.DoorMesh_01`) (`KismetMathLibrary.MakeVector` (+ _returnvalue _door01startpos_x) _door01startpos_y _door01startpos_z) false false)
      (`SceneComponent.K2_SetRelativeLocation` (`self.DoorMesh_02`) (`KismetMathLibrary.MakeVector` (+ (* _returnvalue -1.0) _door02startpos_x) _door02startpos_y _door02startpos_z) false false))))

(event `self.CloseDoor`
  (goto _label :!via `Reverse`))

(fn `UserConstructionScript`
  (`parent.UserConstructionScript`))
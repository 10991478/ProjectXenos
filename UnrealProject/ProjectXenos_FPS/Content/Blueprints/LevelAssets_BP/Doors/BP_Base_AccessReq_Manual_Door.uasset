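; Base Blueprint for a manually operated, access-requirement door that toggles open and closed on signal.
; ActivateSignal runs PostActivation and OpenDoor when the door is closed, or forwards to DeactivateSignal when DoorIsOpen is set.
; DeactivateSignal runs PostDeactivation and CloseDoor, then clears the open flag.
; The access check itself does not appear in these graphs, and construction only calls the parent script.
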(event `/Game/Blueprints/BP_Interfaces/BPI_BasicActivationSignal.ActivateSignal`
  (if (`self.DoorIsOpen`)
    (`self.DeactivateSignal`)
    (else
      (`self.PostActivation`)
      (`self.OpenDoor`)
      (set `self.DoorIsOpen` true))))

(event `/Game/Blueprints/BP_Interfaces/BPI_BasicActivationSignal.DeactivateSignal`
  (`self.PostDeactivation`)
  (`self.CloseDoor`)
  (set `self.DoorIsOpen` false))

(fn `UserConstructionScript`
  (`parent.UserConstructionScript`))
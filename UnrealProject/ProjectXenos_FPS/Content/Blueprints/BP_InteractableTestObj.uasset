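; BP_InteractableTestObj is a test interactable whose cube the player can pick up and drop.
; OnInteract toggles grabbing and releasing the cube through a Physics Handle.
; While held, Tick moves the handle target to a point ahead of the interacting player's root component.
; A collision sphere shows or hides a widget as the first-person character enters or leaves, and IsInteractable always returns false.
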(event `self.ReceiveTick`
  (params (DeltaSeconds :type "Float (single-precision)"))
  ;[1 1 1] Pickup/Drop Interaction
  (if (`self.isGrabbingObject`)
    (bind _rootcomponent (`Actor.RootComponent` (stale `/Game/Blueprints/BP_Interfaces/BPI_Interactable.OnInteract` InteractingPlayer)))
    (`PhysicsHandleComponent.SetTargetLocation` (`self.PhysicsHandle`) (+ (`SceneComponent.K2_GetComponentLocation` _rootcomponent) (* (`KismetMathLibrary.GetForwardVector` (`SceneComponent.K2_GetComponentRotation` _rootcomponent)) 200.0)))))

(event `/Game/Blueprints/BP_Interfaces/BPI_Interactable.OnInteract`
  (params (InteractingPlayer :type "Character Object Reference"))
  (bind _cube (`self.Cube`))
  ;[1 1 1] Pickup/Drop Interaction
  (if (`self.isGrabbingObject`)
    (set `self.isGrabbingObject` false)
    (`PhysicsHandleComponent.ReleaseComponent` (`self.PhysicsHandle`))
    (else
      (set `self.isGrabbingObject` true)
      (`PhysicsHandleComponent.GrabComponentAtLocationWithRotation` :`self` (`self.PhysicsHandle`) :`Component` _cube :`Location` (`SceneComponent.K2_GetComponentLocation` _cube)))))

(event `self. SphereCollision.OnComponentBeginOverlap`
  (params (OverlappedComponent :type "PrimitiveComponent Object Reference") (OtherActor :type "Actor Object Reference") (OtherComp :type "PrimitiveComponent Object Reference") (OtherBodyIndex :type Integer) (bFromSweep :type Boolean) (SweepResult :type "HitResult Structure (by ref)"))
  (cast `/Game/FirstPerson/Blueprints/BP_FirstPersonCharacter` OtherActor)
  (`SceneComponent.SetVisibility` (`self.Widget`) true false))

(event `self. SphereCollision.OnComponentEndOverlap`
  (params (OverlappedComponent :type "PrimitiveComponent Object Reference") (OtherActor :type "Actor Object Reference") (OtherComp :type "PrimitiveComponent Object Reference") (OtherBodyIndex :type Integer))
  (cast `/Game/FirstPerson/Blueprints/BP_FirstPersonCharacter` OtherActor)
  (`SceneComponent.SetVisibility` (`self.Widget`) false false))

(fn `IsInteractable`
  (returns (Interactable :type Boolean))
  (return false))

(fn `UserConstructionScript`)
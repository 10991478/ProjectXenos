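; Base in-hand firearm item that fires projectiles automatically while the user holds it in use and ammo remains.
; UseItem stores the shooter and starts a delayed loop paced by FireRate, which StopUsingItem ends by clearing the Shooting flag.
; Each shot spawns a projectile at the Arrow component, aimed along the shooter's first-person camera, then decrements ammo and clears CanShoot when empty.
; Debug strings print throughout.
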(event `self.UseItem`
  (params (User :type "/Game/FirstPerson/Blueprints/BP_FirstPersonCharacter Object Reference"))
  (`KismetSystemLibrary.PrintString` "started using")
  (set `self.Shooter` User)
  (if (> (`self.CurrentAmmo`) 0)
    (set `self.Shooting` true)
    (`self.Shoot` (`self.Shooter`))))

(event `self.StopUsingItem`
  (params (User :type "/Game/FirstPerson/Blueprints/BP_FirstPersonCharacter Object Reference"))
  (set `self.Shooting` false)
  (`KismetSystemLibrary.PrintString` "stopped using"))

(event `Shoot`
  (params (Shooter :type "/Game/FirstPerson/Blueprints/BP_FirstPersonCharacter Object Reference"))
  (bind _returnvalue (- (`self.CurrentAmmo`) 1))
  (bind _returnvalue_2 (`KismetMathLibrary.Conv_VectorToRotator` (`SceneComponent.GetForwardVector` (`/Game/FirstPerson/Blueprints/BP_FirstPersonCharacter.FirstPersonCamera` Shooter))))
  (`/Game/Blueprints/Macros/BML_BreakAndDelay_Actor.WhileLoopWithBreakAndDelay` (and (`self.Shooting`) (`self.CanShoot`)) (`self.FireRate`)
    (:`LoopBody`
      (`KismetSystemLibrary.PrintString` (`KismetStringLibrary.Concat_StrStr` "Shooting. Current ammo: " (`KismetStringLibrary.Conv_IntToString` (`self.CurrentAmmo`))))
      (bind _returnvalue_3 (`|SpawnActorFromClass` (`self.Projectile`) (`KismetMathLibrary.MakeTransform` (`SceneComponent.K2_GetComponentLocation` (`self.Arrow`)) _returnvalue_2) "AlwaysSpawn" "MultiplyWithRoot" null null))
      (`KismetSystemLibrary.PrintString` (`KismetStringLibrary.Conv_RotatorToString` _returnvalue_2))
      (set `/Game/Blueprints/Items/Firearms/Projectiles/BP_Master_Projectile.Lifespan` (`self.ProjectileLifeSpan`) _returnvalue_3)
      (if (<= _returnvalue 0)
        (set `self.CanShoot` false)
        (set `self.CurrentAmmo` 0)
        (else
          (set `self.CurrentAmmo` _returnvalue))))
    (:`Completed`
      (set `self.Shooting` false))))

(fn `UserConstructionScript`
  (`parent.UserConstructionScript`))
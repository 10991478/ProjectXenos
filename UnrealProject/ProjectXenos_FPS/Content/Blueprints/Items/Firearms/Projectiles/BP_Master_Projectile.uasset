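; BP_Master_Projectile is a firearm projectile, named as a master class, that flies straight along its local X axis until its lifespan runs out.
; On BeginPlay it randomizes speed in both directions and offsets rotation per axis by a random amount between negative AngleVariation and zero.
; Tick moves the Collider with a swept relative offset and destroys the actor once accumulated time reaches Lifespan, with no hit handling in these graphs.
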(event `self.ReceiveBeginPlay`
  (bind (_returnvalue_roll _returnvalue_pitch _returnvalue_yaw) (`KismetMathLibrary.BreakRotator` (`self.K2_GetActorRotation`)))
  (bind _speedvariation (`self.SpeedVariation`))
  (bind (_anglevariation_roll _anglevariation_pitch _anglevariation_yaw) (`KismetMathLibrary.BreakRotator` (`self.AngleVariation`)))
  (set `self.Speed` (+ (`self.Speed`) (`KismetMathLibrary.RandomFloatInRange` (* _speedvariation -1.0) _speedvariation)))
  (`self.K2_SetActorRelativeRotation` (`KismetMathLibrary.MakeRotator` (+ _returnvalue_roll (`KismetMathLibrary.RandomFloatInRange` (* _anglevariation_roll -1.0))) (+ _returnvalue_pitch (`KismetMathLibrary.RandomFloatInRange` (* _anglevariation_pitch -1.0))) (+ _returnvalue_yaw (`KismetMathLibrary.RandomFloatInRange` (* _anglevariation_yaw -1.0))))))

(event `self.ReceiveTick`
  (params (DeltaSeconds :type "Float (single-precision)"))
  (`SceneComponent.K2_AddRelativeLocation` (`self.Collider`) (`KismetMathLibrary.MakeVector` (* DeltaSeconds (`self.Speed`))) true false)
  (bind _output_get (set `self.CurrentLife` (+ DeltaSeconds (`self.CurrentLife`))))
  (if (>= _output_get (`self.Lifespan`))
    (`self.K2_DestroyActor`)))

(fn `UserConstructionScript`)
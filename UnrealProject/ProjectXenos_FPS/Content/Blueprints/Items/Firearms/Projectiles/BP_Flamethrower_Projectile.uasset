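; Flamethrower projectile that can leave a ground fire where it first hits something outside its nonstick classes.
; On collider overlap, a sphere trace supplies the hit location for SpawnFire, along with randomized lifespan and size.
; SpawnFire rolls a stick chance to spawn BP_GroundFire and a second roll to mark its nav modifier as an obstacle area.
; The projectile destroys itself shortly after, whether or not fire spawns.
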(event `self.Collider.OnComponentBeginOverlap`
  (params (OverlappedComponent :type "PrimitiveComponent Object Reference") (OtherActor :type "Actor Object Reference") (OtherComp :type "PrimitiveComponent Object Reference") (OtherBodyIndex :type Integer) (bFromSweep :type Boolean) (SweepResult :type "HitResult Structure (by ref)"))
  (bind _firesizevariation (`self.FireSizeVariation`))
  (bind _firelifespanvariation (`self.FireLifespanVariation`))
  (bind _collider (`self.Collider`))
  (bind _returnvalue (`SceneComponent.K2_GetComponentLocation` _collider))
  (bind _hitlocation (`PrimitiveComponent.K2_SphereTraceComponent` _collider _returnvalue (+ _returnvalue (`SphereComponent.GetScaledSphereRadius` _collider)) 0.0 true false false))
  (if (not (`self.AlreadyHit`))
    (`/Game/Blueprints/Macros/BML_CastToClass_Actor.CastActorToClasses` OtherActor (`self.NonstickClasses`)
      (:`Failed`
        (`self.SpawnFire` _hitlocation (+ (`KismetMathLibrary.RandomFloatInRange` (* _firelifespanvariation -1.0) _firelifespanvariation) (`self.FireLifespan`)) (`KismetMathLibrary.Conv_DoubleToVector` (+ (`KismetMathLibrary.RandomFloatInRange` (* _firesizevariation -1.0) _firesizevariation) 1.0)) (`self.FireStickChance`) (`self.DoesNotFullyBlockPathChance`))
        (set `self.AlreadyHit` true)
        (`KismetSystemLibrary.PrintString` (`KismetStringLibrary.Conv_VectorToString` _hitlocation))))))

(event `SpawnFire`
  (params (Location :type "Vector Structure") (Lifespan :type "Float (double-precision)") (Size :type "Vector Structure" :default (1.0 1.0 1.0)) (SpawnChance :type "Float (double-precision)" :default 1.0) (NotFullBlockageChance :type "Float (double-precision)"))
  (if (<= (`KismetMathLibrary.RandomFloat`) SpawnChance)
    (bind _returnvalue (`|SpawnActorFromClass` "/Game/Blueprints/Items/Firearms/Projectiles/BP_GroundFire.BP_GroundFire_C" (`KismetMathLibrary.MakeTransform` Location (struct) Size) "AlwaysSpawn" "MultiplyWithRoot" null null))
    (set `/Game/Blueprints/Items/Firearms/Projectiles/BP_GroundFire.Lifespan` Lifespan _returnvalue)
    (if (>= (`KismetMathLibrary.RandomFloat`) NotFullBlockageChance)
      (`NavModifierComponent.SetAreaClass` (`/Game/Blueprints/Items/Firearms/Projectiles/BP_GroundFire.NavModifier` _returnvalue) "/Script/NavigationSystem.NavArea_Obstacle"))
    (`KismetSystemLibrary.Delay` 0.1)
    (`self.K2_DestroyActor`)
    (else
      (`KismetSystemLibrary.Delay` 0.1)
      (`self.K2_DestroyActor`))))

(fn `UserConstructionScript`
  (`parent.UserConstructionScript`))
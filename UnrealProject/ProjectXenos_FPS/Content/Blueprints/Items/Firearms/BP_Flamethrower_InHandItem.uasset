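; In-hand flamethrower item that shows a Niagara flame effect while it is being used.
; The flames start inactive and hidden on BeginPlay.
; The UseItemPost event activates and reveals them, and StopUsingItemPost deactivates and hides them again.
; The Blueprint only toggles this effect, with no damage or hit logic of its own.
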(event `self.ReceiveBeginPlay`
  (bind _niagara_flames (`self.Niagara_Flames`))
  (`ActorComponent.SetActive` _niagara_flames false false)
  (`SceneComponent.SetVisibility` _niagara_flames false false))

(event `self.UseItemPost`
  (bind _niagara_flames (`self.Niagara_Flames`))
  (`ActorComponent.SetActive` _niagara_flames true false)
  (`SceneComponent.SetVisibility` _niagara_flames true false))

(event `self.StopUsingItemPost`
  (bind _niagara_flames (`self.Niagara_Flames`))
  (`ActorComponent.SetActive` _niagara_flames false false)
  (`SceneComponent.SetVisibility` _niagara_flames false false))

(fn `UserConstructionScript`
  (`parent.UserConstructionScript`))